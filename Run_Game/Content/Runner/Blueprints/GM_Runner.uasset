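; Game mode for a three-lane runner that builds the track and tracks speed, score and coins.
; After a timed loading screen it chains floor pieces, filling alternate rows with random obstacles, recursively placed coin trails and distance-gated power-ups.
; At most two lanes per row get blocking obstacles.
; Self-repeating events ramp walk speed by shrinking steps outside hyper running and turn X travel into HUD score.
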(event `self.ReceiveBeginPlay`
  (bind _returnvalue (`|CreateWidget` "/Game/Runner/Menu/LoadingScreen.LoadingScreen_C"))
  (`UserWidget.AddToPlayerScreen` _returnvalue 0)
  (`KismetSystemLibrary.Delay` 5.0)
  (`Widget.RemoveFromParent` _returnvalue)
  (set `self.LoadingDone` true)
  (`|ExecutionSequence`
    (:`then_0`
      (bind _outactors (`GameplayStatics.GetAllActorsOfClass` "/Game/Runner/Blueprints/PreFabs/BP_BaseFloor.BP_BaseFloor_C"))
      (bind _output_get (set `self.Base_Floor_Ref` (`|GetArrayItem` _outactors)))
      (set `/Game/Runner/Blueprints/PreFabs/BP_BaseFloor.Game_Mode_Ref` self _output_get)
      (set `self.Next_Spawn_Point` (`SceneComponent.K2_GetComponentLocation` (`/Game/Runner/Blueprints/PreFabs/BP_BaseFloor.SpawnPointNOMOVER` _output_get)))
      (`self.SpawnFloor` 4))
    (:`then_1`
      (`/Engine/EditorBlueprintResources/StandardMacros.IsValid` "/Game/Runner/Blueprints/BP_RunCharacter.BP_RunCharacter" :!label _label
        (:`Is Valid`
          (bind _asbp_run_character (cast `/Game/Runner/Blueprints/BP_RunCharacter` (`GameplayStatics.GetPlayerCharacter` 0)))
          (set `self.Player_Ref` _asbp_run_character))
        (:`Is Not Valid`
          (`KismetSystemLibrary.Delay` 0.01)
          (goto _label))))
    (:`then_2`
      (bind _returnvalue_2 (`|CreateWidget` "/Game/Runner/Blueprints/UI/WBP_PlayerHUD.WBP_PlayerHUD_C"))
      (bind _output_get_2 (set `self.Player_HUD_Ref` _returnvalue_2))
      (`UserWidget.AddToViewport` _output_get_2 0))
    (:`then_3`
      (`self.Increase Speed`))
    (:`then_4`
      (`self.IncreasePoints`))))

(event `Increase Speed`
  (bind _player_ref (`self.Player_Ref`))
  (bind _charactermovement (`Character.CharacterMovement` _player_ref))
  (bind _maxwalkspeed (`CharacterMovementComponent.MaxWalkSpeed` _charactermovement))
  ; Increase Speed
  (if (not (`/Game/Runner/Blueprints/BP_RunCharacter.Hyper_Running?` _player_ref))
    (if (<= _maxwalkspeed 5000.0)
      (set `CharacterMovementComponent.MaxWalkSpeed` (+ _maxwalkspeed (`KismetMathLibrary.MapRangeClamped` _maxwalkspeed 800.0 (`self.Max_Running_Speed`) 100.0 1.0)) _charactermovement)
      (`KismetSystemLibrary.Delay` 1.0)
      (`self.Increase Speed`))))

(event `IncreasePoints`
  (bind _returnvalue_x (`KismetMathLibrary.BreakVector` (`SceneComponent.K2_GetComponentLocation` (`Character.CapsuleComponent` (`self.Player_Ref`)))))
  (set `self.Player_Location_Before` _returnvalue_x)
  (`KismetSystemLibrary.Delay` 0.1)
  (bind _output_get (set `self.Score` (+ (`self.Score`) (/ (- _returnvalue_x (`self.Player_Location_Before`)) 100.0))))
  (`/Game/Runner/Blueprints/UI/WBP_PlayerHUD.UpdatePoints` (`self.Player_HUD_Ref`) _output_get)
  (`self.IncreasePoints`))

(event `IncreaseCoins`
  (params (Amount :type Integer))
  ; Increase Coins
  (bind _output_get (set `self.Coins` (+ Amount (`self.Coins`))))
  (`/Game/Runner/Blueprints/UI/WBP_PlayerHUD.UpdateCoins` (`self.Player_HUD_Ref`) _output_get))

(fn `CoinSpawner`
  (params (Amount :type Integer) (Spawn_After_Location :type "Float (double-precision)" :default 300.0) (Already_Spawing :type Boolean))
  (if Already_Spawing
    (if (> (`self.Coins_Amount_to_Spawn`) 0)
      (`AddComponent|NODE_AddChildActorComponent-3` :`self` (`self.Base_Floor_Ref`) :`RelativeTransform` (`KismetMathLibrary.MakeTransform` (`self.Coin_Spawn_Location`)))
      (`/Engine/EditorBlueprintResources/StandardMacros.DecrementInt` (`self.Coins_Amount_to_Spawn`)
        (:`  `
          (set `self.Coin_Spawn_Location` (+ (`self.Coin_Spawn_Location`) (200.0 0.0 0.0)))
          (`self.CoinSpawner` 0 300.0 true)))
      (else
        (set `self.Coins_Already_Spawn` true)))
    (elif (not (`self.Coins_Already_Spawn`))
      (set `self.Coin_Spawn_Location` (+ (`SceneComponent.RelativeLocation` (`self.Obstacle_Spawn_Point`)) (`KismetMathLibrary.MakeVector` (`local.Spawn_After_Location`) (`self.Obstacle_Lane_Location`))))
      (if (== (`local.Amount`) 0)
        (set `self.Coins_Amount_to_Spawn` (`KismetMathLibrary.RandomIntegerInRange` 1 5))
        (else
          (set `self.Coins_Amount_to_Spawn` (`local.Amount`))))
      (`self.CoinSpawner` 0 300.0 true))))

(fn `MainSpawner`
  (bind _base_floor_ref (`self.Base_Floor_Ref`))
  (for _index (range 6)
    (if (`self.Can_Spawn`)
      (set `self.Obstacle_Spawn_Point` (select `int` _index :`0` (`/Game/Runner/Blueprints/PreFabs/BP_BaseFloor.SpawnLocation1` _base_floor_ref) :`1` (`/Game/Runner/Blueprints/PreFabs/BP_BaseFloor.SpawnLocation2` _base_floor_ref) :`2` (`/Game/Runner/Blueprints/PreFabs/BP_BaseFloor.SpawnLocation3` _base_floor_ref) :`3` (`/Game/Runner/Blueprints/PreFabs/BP_BaseFloor.SpawnLocation4` _base_floor_ref) :`4` (`/Game/Runner/Blueprints/PreFabs/BP_BaseFloor.SpawnLocation5` _base_floor_ref) :`5` (`/Game/Runner/Blueprints/PreFabs/BP_BaseFloor.SpawnLocation6` _base_floor_ref)))
      (`self.SpawnObstacles`)
      (set `self.Can_Spawn` false)
      (else
        (set `self.Can_Spawn` true)))))

(fn `SpawnCoinsAfterObstacle`
  (params (Spawn_Chances :type "Float (double-precision)" :default 33.0) (Spawn_After_Location :type "Float (double-precision)" :default 300.0))
  (if (>= Spawn_Chances (`KismetMathLibrary.RandomFloatInRange` 0.0 100.0))
    (`self.CoinSpawner` 0 (`local.Spawn_After_Location`))))

(fn `SpawnFloor`
  (params (Amount :type Integer))
  ; Spawn Floor
  (for _ (range Amount)
    (bind _returnvalue (`|SpawnActorFromClass` "/Game/Runner/Blueprints/PreFabs/BP_BaseFloor.BP_BaseFloor_C" (`KismetMathLibrary.MakeTransform` (`self.Next_Spawn_Point`)) "Undefined" "MultiplyWithRoot" null null))
    (bind _output_get (set `self.Base_Floor_Ref` _returnvalue))
    (set `/Game/Runner/Blueprints/PreFabs/BP_BaseFloor.Game_Mode_Ref` self _output_get)
    (set `self.Next_Spawn_Point` (`SceneComponent.K2_GetComponentLocation` (`/Game/Runner/Blueprints/PreFabs/BP_BaseFloor.SpawnPointNOMOVER` _output_get)))
    (`self.MainSpawner`)))

(fn `SpawnObstacles`
  (for _index (range 3)
    (set `self.Obstacle_Lane_Location` (select `int` _index :`0` -300.0 :`1` 0.0 :`2` 300.0))
    (switch `int` (`KismetMathLibrary.RandomIntegerInRange` 0 5)
      (:`0`
        (`AddComponent|NODE_AddChildActorComponent-0` :`self` (`self.Base_Floor_Ref`) :`RelativeTransform` (`KismetMathLibrary.MakeTransform` (+ (`SceneComponent.RelativeLocation` (`self.Obstacle_Spawn_Point`)) (`KismetMathLibrary.MakeVector` 0.0 (`self.Obstacle_Lane_Location`)))))
        (`self.SpawnCoinsAfterObstacle` 33.0)
        (`self.SpawnPowerUps` false 300.0 10.0))
      (:`1`
        (`AddComponent|NODE_AddChildActorComponent-2` :`self` (`self.Base_Floor_Ref`) :`RelativeTransform` (`KismetMathLibrary.MakeTransform` (+ (`SceneComponent.RelativeLocation` (`self.Obstacle_Spawn_Point`)) (`KismetMathLibrary.MakeVector` 0.0 (`self.Obstacle_Lane_Location`)))))
        (`self.SpawnCoinsAfterObstacle` 33.0)
        (`self.SpawnPowerUps` false 1000.0 10.0))
      (:`2`
        (if (< (`self.Lanes_Blocked`) 2)
          (`AddComponent|NODE_AddChildActorComponent-1` :`self` (`self.Base_Floor_Ref`) :`RelativeTransform` (`KismetMathLibrary.MakeTransform` (+ (`SceneComponent.RelativeLocation` (`self.Obstacle_Spawn_Point`)) (`KismetMathLibrary.MakeVector` 0.0 (`self.Obstacle_Lane_Location`)))))
          (`/Engine/EditorBlueprintResources/StandardMacros.IncrementInt` (`self.Lanes_Blocked`))))
      (:`3`
        (if (< (`self.Lanes_Blocked`) 2)
          (`AddComponent|NODE_AddChildActorComponent-10` :`self` (`self.Base_Floor_Ref`) :`RelativeTransform` (`KismetMathLibrary.MakeTransform` (+ (`SceneComponent.RelativeLocation` (`self.Obstacle_Spawn_Point`)) (`KismetMathLibrary.MakeVector` 0.0 (`self.Obstacle_Lane_Location`)))))
          (`/Engine/EditorBlueprintResources/StandardMacros.IncrementInt` (`self.Lanes_Blocked`))))
      (:`4`
        (`self.CoinSpawner` 0 0.0))))
  (set `self.Lanes_Blocked` 0)
  (set `self.Coins_Already_Spawn` false)
  (set `self.Power_Up_Already_Spawned` false)
  (`/Engine/EditorBlueprintResources/StandardMacros.IncrementInt` (`self.Power_Up_Distance_From_Last`)))

(fn `SpawnPowerUps`
  (params (Force_Spawn :type Boolean) (Spawn_After_Location :type "Float (double-precision)" :default 300.0) (Power_Up_Spawn_Chance :type "Float (double-precision)" :default 5.0) (Select_Power_Up :type Boolean) (Power_Up_Index :type Integer))
  (if (not (`self.Power_Up_Already_Spawned`))
    (if Force_Spawn
      (switch `int` (`KismetMathLibrary.SelectInt` (`local.Power_Up_Index`) (`KismetMathLibrary.RandomIntegerInRange` 0 1) (`local.Select_Power_Up`)) :!label _label
        (:`0`
          (`AddComponent|NODE_AddChildActorComponent-5` :`self` (`self.Base_Floor_Ref`) :`RelativeTransform` (`KismetMathLibrary.MakeTransform` (+ (`SceneComponent.RelativeLocation` (`self.Obstacle_Spawn_Point`)) (`KismetMathLibrary.MakeVector` (`local.Spawn_After_Location`) (`self.Obstacle_Lane_Location`)))))
          (set `self.Power_Up_Already_Spawned` true)
          (set `self.Power_Up_Distance_From_Last` 0))
        (:`1`
          (`AddComponent|NODE_AddChildActorComponent-6` :`self` (`self.Base_Floor_Ref`) :`RelativeTransform` (`KismetMathLibrary.MakeTransform` (+ (`SceneComponent.RelativeLocation` (`self.Obstacle_Spawn_Point`)) (`KismetMathLibrary.MakeVector` (`local.Spawn_After_Location`) (`self.Obstacle_Lane_Location`)))))
          (set `self.Power_Up_Already_Spawned` true)
          (set `self.Power_Up_Distance_From_Last` 0)))
      (elif (>= (`self.Power_Up_Distance_From_Last`) (`self.Power_up_Minimun_Distance`))
        (if (>= (`local.Power_Up_Spawn_Chance`) (`KismetMathLibrary.RandomFloatInRange` 0.0 100.0))
          (goto _label))))))

(fn `UserConstructionScript`)