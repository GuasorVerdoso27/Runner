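; Player camera for a lane-based runner that follows the player along X and shifts sideways between three lanes.
; Each Tick it places the camera at the player capsule's X plus the FollowLocation offset, at FollowLocation's fixed Z.
; CalculateLaneLocation eases Y toward the LaneIndex lane using FInterpTo at the player's lane switch speed.
; That interpolated Y is returned only while the player's lane is not blocked.
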(event `self.ReceiveTick`
  (params (DeltaSeconds :type "Float (single-precision)"))
  (bind _follow_location (`self.Follow_Location`))
  (bind _returnvalue_x (`KismetMathLibrary.BreakVector` (`SceneComponent.K2_GetComponentLocation` (`Character.CapsuleComponent` (`self.Player_Ref`)))))
  ; Set Camera to player
  (`SceneComponent.K2_SetWorldLocation` (`self.CameraComponent`) (`KismetMathLibrary.MakeVector` (+ _returnvalue_x (.x (.location _follow_location))) (`self.CalculateLaneLocation`) (.z (.location _follow_location))) false false))

(fn `CalculateLaneLocation`
  (returns (Lane_Location :type "Float (double-precision)"))
  (bind _move_amount (`self.Move_Amount`))
  (bind (_returnvalue_x _returnvalue_y) (`KismetMathLibrary.BreakVector` (`SceneComponent.K2_GetComponentLocation` (`self.CameraComponent`))))
  ; Set Lane Camera location
  (if (not (`/Game/Runner/Blueprints/BP_RunCharacter.Lane_blocked` (`self.Player_Ref`)))
    (return (`KismetMathLibrary.FInterpTo` _returnvalue_y (select `int` (`self.Lane_Index`) :`0` (* _move_amount -1.0) :`1` 1.0 :`2` _move_amount) (`GameplayStatics.GetWorldDeltaSeconds`) (`/Game/Runner/Blueprints/BP_RunCharacter.GetLaneSwitchSpeed` (`self.Player_Ref`))))))

(fn `UserConstructionScript`)