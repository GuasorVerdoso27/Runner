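; BP_Vive100 is a runner pickup that opens a slow-motion special challenge when BP_RunCharacter touches it.
; It hides, dilates time to a tenth and plays looping step sounds while a timer counts until timeout or the character ends the special.
; Failure prints a message and destroys it.
; Otherwise it temporarily boosts walk speed and GM_Runner's max speed with HyperRunning, then restores them, calls IncreaseSpeed and destroys itself.
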(event `self.Collision.OnComponentBeginOverlap`
  (params (OverlappedComponent :type "PrimitiveComponent Object Reference") (OtherActor :type "Actor Object Reference") (OtherComp :type "PrimitiveComponent Object Reference") (OtherBodyIndex :type Integer) (bFromSweep :type Boolean) (SweepResult :type "HitResult Structure (by ref)"))
  (bind _asbp_run_character (cast `/Game/Runner/Blueprints/BP_RunCharacter` OtherActor))
  (bind _output_get (set `self.Player_Ref` _asbp_run_character))
  (set `/Game/Runner/Blueprints/BP_RunCharacter.Is_Special_Active` true _output_get)
  (bind _output_get_2 (set `self.Old_Speed` (`CharacterMovementComponent.MaxWalkSpeed` (`Character.CharacterMovement` _output_get))))
  (set `self.New_Speed` (+ _output_get_2 1000.0))
  (`SceneComponent.SetVisibility` (`self.vive100`) false false)
  (`GameplayStatics.PlaySoundAtLocation` "/Game/Runner/Audio/power.power" (`self.K2_GetActorLocation`) (struct) 1.0 1.0 0.0 null null null null)
  (`self.SpecialCounter`)
  (`KismetSystemLibrary.K2_SetTimerDelegate` (delegate `SpecialCounter`) 0.1 true)
  (`GameplayStatics.SetGlobalTimeDilation` 0.1))

(event `SpecialCounter`
  (bind _old_speed (`self.Old_Speed`))
  (bind _player_ref (`self.Player_Ref`))
  (bind _charactermovement (`Character.CharacterMovement` _player_ref))
  (if (or (>= (`self.Time_Elapsed`) 3) (not (`/Game/Runner/Blueprints/BP_RunCharacter.Is_Special_Active` (`self.Player_Ref`))))
    (`GameplayStatics.SetGlobalTimeDilation` 1.0)
    (set `/Game/Runner/Blueprints/BP_RunCharacter.Is_Special_Active` false (`self.Player_Ref`))
    (if (`/Game/Runner/Blueprints/BP_RunCharacter.Special_Failed` (`self.Player_Ref`))
      (`KismetSystemLibrary.PrintString` "No lo lograste")
      (`self.K2_DestroyActor`)
      (else
        (set `/Game/Runner/Blueprints/BP_RunCharacter.Hyper_Running?` true _player_ref)
        (bind _output_get (set `CharacterMovementComponent.MaxWalkSpeed` (`self.New_Speed`) _charactermovement))
        (bind _asgm_runner (cast `/Game/Runner/Blueprints/GM_Runner` (`GameplayStatics.GetGameMode`)))
        (set `/Game/Runner/Blueprints/GM_Runner.Max_Running_Speed` _output_get _asgm_runner)
        (`KismetSystemLibrary.Delay` 3.0)
        (`KismetSystemLibrary.PrintString` (`KismetStringLibrary.Conv_DoubleToString` _old_speed))
        (set `CharacterMovementComponent.MaxWalkSpeed` _old_speed _charactermovement)
        (set `/Game/Runner/Blueprints/GM_Runner.Max_Running_Speed` 5000.0 _asgm_runner)
        (set `/Game/Runner/Blueprints/BP_RunCharacter.Hyper_Running?` false (`self.Player_Ref`))
        (`/Game/Runner/Blueprints/GM_Runner.Increase Speed` _asgm_runner)
        (`self.K2_DestroyActor`)))
    (else
      (bind _result (`/Engine/EditorBlueprintResources/StandardMacros.IncrementInt` (`self.Time_Elapsed`))
        (:`  `
          (`self.PlaySound`)
          (`KismetSystemLibrary.K2_SetTimerDelegate` (delegate `PlaySound`) 0.05 true))))))

(event `PlaySound`
  (`GameplayStatics.PlaySoundAtLocation` "/Game/Runner/Audio/MSS_pasos.MSS_pasos" (`self.K2_GetActorLocation`) (struct) 5.0 1.0 0.0 null null null null))

(fn `CompleteSpecial`)

(fn `UserConstructionScript`)